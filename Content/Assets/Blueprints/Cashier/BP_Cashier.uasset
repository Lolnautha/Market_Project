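; Cashier station actor that toggles the player between first-person and cashier controls by swapping Enhanced Input mapping contexts.
; In cashier mode, look input rotates a clamped camera and line-traces the component under view, storing it as Button.
; Helpers set cursor visibility from the game instance and turn appended digits into a decimal total.
; A debug key spawns a Chips product box from a data table at the delivery area.
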(event Input|EnhancedActionEvents|EnhancedInputActionIA_Look
  (params (ActionValue :type Vector%202D%20Structure) (ElapsedSeconds :type Float%20%28double-precision%29) (TriggeredSeconds :type Float%20%28double-precision%29) (InputAction :type Input%20Action%20Object%20Reference :default "/Game/Input/Player/Actions/IA_Look.IA_Look"))
  (bind _camera (Variables|Default|GetCamera))
  (bind _camera_2 (Variables|Default|GetCamera))
  (bind _returnvalue (Transformation|GetWorldLocation _camera))
  (bind _returnvalue_2 (Transformation|GetWorldRotation _camera_2))
  ;[0 0 0] (Cashier) Check Cashier Event
  (if (Variables|Default|GetisCashierEvent)
    ;[0.005208 0.005208 0.005208] (Cashier) Camera rotation
    (Transformation|SetWorldRotation (Variables|Default|GetCamera) (Math|Rotator|MakeRotator 0.0 (Math|Float|Clamp(Float) (+ (.pitch _returnvalue_2) (* (.y ActionValue) (Variables|Camera|GetsensVertical) -1.0 0.75)) -7e+01 5.0) (Math|Float|Clamp(Float) (+ (.yaw _returnvalue_2) (* (.x ActionValue) (Variables|Camera|GetsensHorizontal) 0.75)) -6e+01 6e+01)) false false)
    ;[0 0 0] (Cashier) Store raycasting
    (bind _returnvalue_3 (Actor|GetActorOfClass 0))
    (bind _outhit (Collision|LineTraceByChannel _returnvalue (+ _returnvalue (* (Math|Vector|GetForwardVector _camera) 3e+02)) "TraceTypeQuery1" true (Utilities|Array|MakeArray _returnvalue_3) "ForOneFrame" false))
    (Variables|Raycast|SetButton (.HitComponent (Collision|BreakHitResult _outhit)))))

(event EventBeginPlay
  (bind _camera (Variables|Default|GetCamera))
  ;[0 0 0] (Begin play)
  ;[0 0 0] (Player) Set the player to the desire location
  (Transformation|SetWorldLocation _camera (Transformation|GetWorldLocation (Variables|Default|GetCameraPosition)) false true)
  (Variables|Camera|SetCameraIniRot (Transformation|GetWorldRotation _camera)))

(event EventCashierFunction
  ;[0 0 0] (Cashier) When possesing the actor, the mapping will be replace to the cashier input mapping
  (if (.ReturnValue (Class|EnhancedInputSubsystemInterface|HasMappingContext (PlayerController|LocalPlayerSubsystems|GetEnhancedInputLocalPlayerSubsystem (Game|GetPlayerController 0)) "/Game/Input/Cashier/Mapping/IMC_Cashier.IMC_Cashier"))
    (|removeMapping)
    (Variables|Default|SetisCashierEvent false)
    (Transformation|SetWorldRotation (Variables|Default|GetCamera) (Variables|Camera|GetCameraIniRot) false false)
    (else
      (|addMapping)
      (Variables|Default|SetisCashierEvent true))))

(event Input|KeyboardEvents|DebugKeyF
  (params (Key :type Key%20Structure :default "None") (ActionValue :type Input%20Action%20Value%20Structure))
  (bind _returnvalue (Utilities|String|MakeLiteralString "Chips"))
  (:Pressed
    (bind _returnvalue_2 (Utilities|GetDataTableRow (Variables|Default|GetData%20Products) (Utilities|String|StringToName _returnvalue))
      (:then
        (bind _returnvalue_3 (Game|SpawnActorfromClass (.Product_Box (Utilities|Struct|BreakS_ProductsData _returnvalue_2)) (Transformation|GetActorTransform (Utilities|ResolveSoftReference (Variables|Default|GetDeliveryArea))) "Undefined" "MultiplyWithRoot" 0 0))
        (bind _asbp_box_of_products (Utilities|Casting|CastToBP_BoxOfProducts _returnvalue_3))
        (Variables|/Game/Assets/Blueprints/CardboardBox/BP_BoxOfProducts.BP_BoxOfProducts_C|SetB_Name _asbp_box_of_products (Utilities|String|StringToName _returnvalue))
        (Variables|/Game/Assets/Blueprints/CardboardBox/BP_BoxOfProducts.BP_BoxOfProducts_C|SetB_Quant _asbp_box_of_products (.Product_Amount (Utilities|Struct|BreakS_ProductsData _returnvalue_2)))
        (Variables|/Game/Assets/Blueprints/CardboardBox/BP_BoxOfProducts.BP_BoxOfProducts_C|SetB_Gone _asbp_box_of_products (.Product_Gone (Utilities|Struct|BreakS_ProductsData _returnvalue_2)))
        (Variables|/Game/Assets/Blueprints/CardboardBox/BP_BoxOfProducts.BP_BoxOfProducts_C|SetB_Product _asbp_box_of_products (.Product_Product (Utilities|Struct|BreakS_ProductsData _returnvalue_2)))
        (Variables|/Game/Assets/Blueprints/CardboardBox/BP_BoxOfProducts.BP_BoxOfProducts_C|SetB_Value _asbp_box_of_products (.Product_Value (Utilities|Struct|BreakS_ProductsData _returnvalue_2)))))))

(fn ConstructionScript)

(fn EnableMouseCamera
  (bind _returnvalue (Game|GetPlayerController 0))
  (bind _ascustom_game_instance (Utilities|Casting|CastToCustom_GameInstance (Game|GetGameInstance)))
  (if (Variables|/Game/Assets/GameInstance/Custom_GameInstance.Custom_GameInstance_C|GetCashier_MouseCheck _ascustom_game_instance)
    (bind _output_get (Variables|/Script/Engine.PlayerController|SetbShowMouseCursor _returnvalue false))
    (bind _output_get_2 (Variables|/Script/Engine.PlayerController|SetbEnableClickEvents _returnvalue _output_get))
    (Variables|/Script/Engine.PlayerController|SetbEnableMouseOverEvents _returnvalue _output_get_2)
    (else
      (bind _output_get_3 (Variables|/Script/Engine.PlayerController|SetbShowMouseCursor _returnvalue true))
      (bind _output_get_4 (Variables|/Script/Engine.PlayerController|SetbEnableClickEvents _returnvalue _output_get_3))
      (Variables|/Script/Engine.PlayerController|SetbEnableMouseOverEvents _returnvalue _output_get_4)))
  (Input|SetInputModeGameOnly _returnvalue (Variables|Default|GetisCashierEvent)))

(fn AddingNumbers
  (params (B :type String))
  (bind _output_get (Variables|CashierMathFunc|SetStringValue (Utilities|String|Append (Variables|CashierMathFunc|GetStringValue) B)))
  (Variables|CashierMathFunc|SetTotalValue (/ (Math|Conversions|ToFloat(Integer) _output_get) 1e+02)))